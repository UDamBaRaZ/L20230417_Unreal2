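; BP_P38 is a P-38 plane actor that flies steadily forward and spins its two propellers.
; Each Tick adds a frame-time-scaled local X offset at a hardcoded speed, then calls NewFunction for the Left and Right propellers.
; NewFunction rolls the given component by PropellerRotateSpeed times delta time.
; Disconnected nodes hold alternative movement versions, including the only use of MaxSpeed, and never run.
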(event EventBeginPlay)

(event EventTick
  (params (DeltaSeconds :type Float%20%28single-precision%29))
  ;[1 1 1] 비행기의 전면으로 이동1
  (Transformation|AddActorLocalOffset (Math|Vector|MakeVector (* (Utilities|Time|GetWorldDeltaSeconds) 1e+02) 0.0 0.0) false false)
  ;[1 1 1] 왼쪽 프로펠러 회전
  (CallFunction|NewFunction (Variables|Default|GetLeft))
  ;[1 1 1] 오른쪽 프로펠러 회전
  (CallFunction|NewFunction (Variables|Default|GetRight)))

(fn ConstructionScript)

(fn NewFunction
  (params (Where :type Static%20Mesh%20Component%20Object%20Reference))
  (Transformation|AddRelativeRotation Where (Math|Rotator|MakeRotator (* (Utilities|Time|GetWorldDeltaSeconds) (Variables|속도|GetPropeller_Rotate_Speed)) 0.0 0.0) false false))